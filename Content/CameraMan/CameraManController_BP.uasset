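; Player controller for a free camera pawn, adapted from the turn-based strategy template, handling mouse rotation and WASD movement.
; Holding right mouse opens a Tick gate that adds scaled mouse delta to control rotation and applies only yaw to the pawn.
; Right and Forward axes share one SetActorLocation, moving the pawn along its root's right and forward vectors by MoveSpeed at constant height, without sweep or delta-time scaling.
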(event `self.ReceiveTick`
  (params (DeltaSeconds :type "Float (single-precision)"))
  (bind (_deltax _deltay) (`self.GetInputMouseDelta`))
  (bind _yaw (.yaw (`self.GetControlRotation`)))
  ;[1 1 1] Camera Rotation from turn based strategy template
  (`/Engine/EditorBlueprintResources/StandardMacros.Gate` true :!label _label
    (:`Exit`
      (`self.K2_SetActorRotation` (`self.K2_GetPawn`) (`KismetMathLibrary.MakeRotator` 0.0 0.0 _yaw) false)
      (`self.SetControlRotation` (`KismetMathLibrary.MakeRotator` (.roll (`self.GetControlRotation`)) (+ (.pitch (`self.GetControlRotation`)) (* _deltay 4.0)) (+ _yaw (* _deltax 4.0)))))))

(event `Key|RightMouseButton`
  (params (Key :type "Key Structure"))
  ;[1 1 1] Camera Rotation from turn based strategy template
  (:`Pressed`
    (goto _label :!via `Open`))
  (:`Released`
    (goto _label :!via `Close`)))

(event `InputAxis|Right`
  (params (AxisValue :type "Float (single-precision)"))
  (bind _returnvalue (`self.K2_GetPawn`))
  ;[1 1 1] WASD movement, foward + back, and Strafe Left + Right from turn based strategy template
  (`self.K2_SetActorLocation` (`self.K2_GetPawn`) (`KismetMathLibrary.MakeVector` (.x (+ (`self.K2_GetActorLocation` (`self.K2_GetPawn`)) (+ (* (`KismetMathLibrary.GetRightVector` (`SceneComponent.K2_GetComponentRotation` (`self.K2_GetRootComponent` _returnvalue))) (* AxisValue (`self.MoveSpeed`))) (* (`KismetMathLibrary.GetForwardVector` (`SceneComponent.K2_GetComponentRotation` (`self.K2_GetRootComponent` _returnvalue))) (* (stale `InputAxis|Forward` AxisValue) (`self.MoveSpeed`)))))) (.y (+ (`self.K2_GetActorLocation` (`self.K2_GetPawn`)) (+ (* (`KismetMathLibrary.GetRightVector` (`SceneComponent.K2_GetComponentRotation` (`self.K2_GetRootComponent` _returnvalue))) (* AxisValue (`self.MoveSpeed`))) (* (`KismetMathLibrary.GetForwardVector` (`SceneComponent.K2_GetComponentRotation` (`self.K2_GetRootComponent` _returnvalue))) (* (stale `InputAxis|Forward` AxisValue) (`self.MoveSpeed`)))))) (.z (`self.K2_GetActorLocation` _returnvalue))) false false :!label _label_2))

(event `InputAxis|Forward`
  (params (AxisValue :type "Float (single-precision)"))
  ;[1 1 1] WASD movement, foward + back, and Strafe Left + Right from turn based strategy template
  (goto _label_2))

(fn `UserConstructionScript`)