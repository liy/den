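; Guest_BP is an AI guest character with its own wallet for making payments.
; The construction script gives each guest a random maximum walk speed, so guests move at varied paces.
; Pay deducts a cost only if money remains afterward, prints the new balance and returns whether it succeeded, so spending the exact balance fails.
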(fn `Pay`
  (params (Cost :type "Float (double-precision)"))
  (returns (CanPay :type Boolean))
  (if (> (- (`self.Wallet`) Cost) 0.0)
    (bind _output_get (set `self.Wallet` (- (`self.Wallet`) Cost)))
    (`KismetSystemLibrary.PrintString` (`KismetStringLibrary.Conv_DoubleToString` _output_get))
    (return true)
    (else
      (return false))))

(fn `UserConstructionScript`
  (set `CharacterMovementComponent.MaxWalkSpeed` (`KismetMathLibrary.RandomFloatInRange` 250.0 500.0) (`self.CharacterMovement`)))